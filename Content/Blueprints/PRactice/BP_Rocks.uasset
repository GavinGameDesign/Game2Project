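; BP_Rocks is a rock actor that makes itself known to the third-person character when nearby.
; Its Sphere overlap passes the rock to BP_ThirdPersonCharacter through SetNearbyRock on entry and clears that reference on exit.
; On BeginPlay it rolls a random Strength from a range chosen by RockType.
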(event OnComponentBeginOverlap(Sphere)
  (params (OverlappedComponent :type Primitive%20Component%20Object%20Reference) (OtherActor :type Actor%20Object%20Reference) (OtherComp :type Primitive%20Component%20Object%20Reference) (OtherBodyIndex :type Integer) (bFromSweep :type Boolean) (SweepResult :type Hit%20Result%20Structure%20%28by%20ref%29))
  (bind _asbp_third_person_character (Utilities|Casting|CastToBP_ThirdPersonCharacter OtherActor))
  (Default|SetNearbyRock _asbp_third_person_character self))

(event OnComponentEndOverlap(Sphere)
  (params (OverlappedComponent :type Primitive%20Component%20Object%20Reference) (OtherActor :type Actor%20Object%20Reference) (OtherComp :type Primitive%20Component%20Object%20Reference) (OtherBodyIndex :type Integer))
  (bind _asbp_third_person_character (Utilities|Casting|CastToBP_ThirdPersonCharacter OtherActor))
  (Default|SetNearbyRock _asbp_third_person_character))

(event EventBeginPlay
  (switch int (Variables|Default|GetRockType)
    (:0
      (Variables|Default|SetStrength (Math|Random|RandomIntegerinRange 5 8)))
    (:1
      (Variables|Default|SetStrength (Math|Random|RandomIntegerinRange 3 5)))
    (:2
      (Variables|Default|SetStrength (Math|Random|RandomIntegerinRange 2 3)))))

(fn ConstructionScript)