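; BP_EnemyTester is a test actor that repeatedly damages every BP_Enemy in the level.
; On BeginPlay it finds all enemies, prints their count, calls TakeDamage on each with a small random amount and prints a confirmation.
; After a two-second delay it calls its GetDamage event, which wires back to the start, so the search and damage pass loops indefinitely.
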(event Custom|Get%20Damage
  (bind _outactors (Actor|GetAllActorsOfClass "/Game/Blueprints/PRactice/BP_Enemy.BP_Enemy_C"))
  (Development|PrintString (Utilities|String|Append "There are " (Utilities|String|ToString(Integer) (Utilities|Array|Length _outactors)) " enemies in the level"))
  (for _array_element _outactors
    (Default|TakeDamage _array_element (Math|Random|RandomFloatinRange 0.1 0.5)))
  (Development|PrintString "All enemies emotionally damaged")
  (Utilities|FlowControl|Delay 2.0)
  (CallFunction|GetDamage))

(event EventBeginPlay
  (bind _outactors (Actor|GetAllActorsOfClass "/Game/Blueprints/PRactice/BP_Enemy.BP_Enemy_C"))
  (Development|PrintString (Utilities|String|Append "There are " (Utilities|String|ToString(Integer) (Utilities|Array|Length _outactors)) " enemies in the level"))
  (for _array_element _outactors
    (Default|TakeDamage _array_element (Math|Random|RandomFloatinRange 0.1 0.5)))
  (Development|PrintString "All enemies emotionally damaged")
  (Utilities|FlowControl|Delay 2.0)
  (CallFunction|GetDamage))

(fn ConstructionScript)