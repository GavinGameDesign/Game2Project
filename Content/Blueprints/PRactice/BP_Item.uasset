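; BP_Item is a holdable item Actor that can be picked up, dropped and used.
; Pickup disables ParentCube collision and snaps the item to the given mesh's item_r socket.
; Drop detaches it and simulates physics for a short delay, then freezes it and restores query and physics collision.
; PrimaryAction switches on ItemIndex but only prints placeholder break, chop or dig messages.
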(event Custom|PrimaryAction
  (switch int (Variables|Components|GetItemIndex)
    (:0
      (Development|PrintString "Break Break"))
    (:1
      (Development|PrintString "Chop Chop"))
    (:2
      (Development|PrintString "Dig Dig"))))

(event Custom|Pickup
  (params (Mesh :type Scene%20Component%20Object%20Reference))
  (Collision|SetCollisionEnabled (Variables|Default|GetParentCube) "NoCollision")
  (Transformation|AttachComponentToComponent Mesh "item_r" "SnapToTarget" "SnapToTarget" "KeepRelative" true))

(event Custom|Drop
  (bind _parentcube (Variables|Default|GetParentCube))
  (Collision|SetCollisionEnabled (Variables|Default|GetParentCube) "PhysicsOnly")
  (Transformation|DetachFromComponent (Variables|Default|GetParentCube) "KeepWorld" "KeepWorld" "KeepWorld" true)
  (Physics|SetSimulatePhysics (Variables|Default|GetParentCube) true)
  (Utilities|FlowControl|Delay 2.0)
  (Physics|SetSimulatePhysics _parentcube false)
  (Collision|SetCollisionEnabled _parentcube "QueryAndPhysics"))

(fn ConstructionScript)