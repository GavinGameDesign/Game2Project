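; BP_Axe is an axe tool whose primary action harvests wood from a nearby tree.
; Each use finds BP_ResourceManager with GetActorOfClass and increments its Oak, Maple or Beech amount according to the tree's type.
; The hit also decrements the tree's Strength, destroys it at zero, then calls Update on the resource manager.
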(event EventPrimaryAction
  (params (NearbyRock :type BP%20Rocks%20Object%20Reference) (NearbyTree :type BP%20Trees%20Object%20Reference))
  (Utilities|IsValid NearbyTree
    (:Is%20Valid
      (bind _output_get (Variables|Default|SetNearbyTree NearbyTree))
      (bind _returnvalue (Actor|GetActorOfClass "/Game/Blueprints/PRactice/Widgets/BP_ResourceManager.BP_ResourceManager_C"))
      (switch int (Variables|/Game/Blueprints/PRactice/BP_Trees.BP_Trees_C|GetTreeType _output_get)
        (:0
          (Math|Integer|IncrementInt (Variables|/Game/Blueprints/PRactice/Widgets/BP_ResourceManager.BP_ResourceManager_C|GetOakAmount _returnvalue)
            (:%20%20
              _)))
        (:1
          (Math|Integer|IncrementInt (Variables|/Game/Blueprints/PRactice/Widgets/BP_ResourceManager.BP_ResourceManager_C|GetMapleAmount _returnvalue)
            (:%20%20
              _)))
        (:2
          (Math|Integer|IncrementInt (Variables|/Game/Blueprints/PRactice/Widgets/BP_ResourceManager.BP_ResourceManager_C|GetBeechAmount _returnvalue)
            (:%20%20
              _))))
      (bind _result (Math|Integer|DecrementInt (Variables|/Game/Blueprints/PRactice/BP_Trees.BP_Trees_C|GetStrength _output_get))
        (:%20%20
          (if (== _result 0)
            (Actor|DestroyActor (Variables|Default|GetNearbyTree)))
          (Default|Update _returnvalue))))))

(fn ConstructionScript
  (|CallParentFunction))